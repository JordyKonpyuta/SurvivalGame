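; Game state for a multiplayer survival game that relays group invites, fast-travel requests and chat through player controllers.
; On BeginPlay it copies travel locations and the map camera to player states.
; It keeps one group list, firing a change event on add and RepNotify, and forwards teleport requests to its other members.
; Group chat instead reaches every player whose own state lists them as grouped, regardless of sender.
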(event `self.ReceiveBeginPlay`
  (`self.S_SetTravelLocations`))

(event `S_SendGroupRequest`
  (params (PlayerThatReceiveInvit :type "PlayerState Object Reference") (PlayerThatSendRequest :type "PlayerState Object Reference"))
  ; Group request Events
  (`/Game/StarterPack/ThirdPerson/Blueprints/BP_ThirdPersonPlayerController.OC_SendGroupRequest` (cast `/Game/StarterPack/ThirdPerson/Blueprints/BP_ThirdPersonPlayerController` (`PlayerState.GetPlayerController` PlayerThatReceiveInvit) :!pure true) PlayerThatReceiveInvit PlayerThatSendRequest))

(event `S_AddPlayerToGroup`
  (params (PlayerThatSendRequest :type "PlayerState Object Reference") (PlayerToAdd :type "PlayerState Object Reference"))
  ; Group request Events
  (`KismetArrayLibrary.Array_AddUnique` (`self.PlayersInGroup`) PlayerThatSendRequest)
  (`KismetArrayLibrary.Array_AddUnique` (`self.PlayersInGroup`) PlayerToAdd)
  (`self.OnGroupChanged`))

(event `S_SetTravelLocations`
  ; Fast Travel Events
  (for _array_element (`self.PlayerArray`)
    (bind _asbp_custom_player_state (cast `/Game/SurvivalGame/BP_CustomPlayerState` _array_element :!pure true))
    (`/Engine/EditorBlueprintResources/StandardMacros.IsValid` _asbp_custom_player_state
      (:`Is Valid`
        (set `/Game/SurvivalGame/BP_CustomPlayerState.TravelLocations` (`self.TravelLocations`) _asbp_custom_player_state)
        (set `/Game/SurvivalGame/BP_CustomPlayerState.MapCamera` (`self.MapCamera`) _asbp_custom_player_state)))))

(event `S_SendTeleportRequest`
  (params (LocationToTravel :type "/Game/SurvivalGame/GroupSystem/BP_Tag Object Reference") (PlayerThatSendRequest :type "PlayerState Object Reference"))
  ; Fast Travel Events
  (if (> (`KismetArrayLibrary.Array_Length` (`self.PlayersInGroup`)) 0)
    (for _array_element (`self.PlayersInGroup`)
      (if (!= _array_element PlayerThatSendRequest)
        (`/Game/StarterPack/ThirdPerson/Blueprints/BP_ThirdPersonPlayerController.OC_ReceiveTeleportRequest` (cast `/Game/StarterPack/ThirdPerson/Blueprints/BP_ThirdPersonPlayerController` (`PlayerState.GetPlayerController` _array_element) :!pure true) LocationToTravel PlayerThatSendRequest)))))

(event `S_ChatToAll`
  (params (TextToSend :type Text) (Sender :type "PlayerState Object Reference"))
  ; Chat Events
  (for _array_element (`self.PlayerArray`)
    (`self.S_RequestMessage` _array_element TextToSend false Sender)))

(event `S_RequestMessage`
  (params (PlayerToSend :type "PlayerState Object Reference") (TextSend :type Text) (IsFromGroup :type Boolean) (Sender :type "PlayerState Object Reference"))
  (`/Game/StarterPack/ThirdPerson/Blueprints/BP_ThirdPersonPlayerController.OC_ReceiveMessage` (cast `/Game/StarterPack/ThirdPerson/Blueprints/BP_ThirdPersonPlayerController` (`PlayerState.GetPlayerController` PlayerToSend) :!pure true) TextSend IsFromGroup Sender))

(event `S_ChatToGroup`
  (params (TextToSend :type Text) (Sender :type "PlayerState Object Reference"))
  ; Chat Events
  (for _array_element (`self.PlayerArray`)
    (if (`KismetArrayLibrary.Array_Contains` (`/Game/SurvivalGame/BP_CustomPlayerState.PlayersInGroup` (cast `/Game/SurvivalGame/BP_CustomPlayerState` _array_element :!pure true)) (cast `/Game/SurvivalGame/BP_CustomPlayerState` _array_element :!pure true))
      (`self.S_RequestMessage` _array_element TextToSend true Sender))))

(fn `OnRep_PlayersInGroup`
  (`self.OnGroupChanged`))

(fn `UserConstructionScript`)