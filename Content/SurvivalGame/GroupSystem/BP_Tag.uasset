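; BP_Tag is a world location marker that serves as a discoverable travel location and player checkpoint.
; On BeginPlay it registers in the game state's TravelLocations and links itself to its WBP_Tag widget, whose visibility can be toggled.
; When a locally controlled character enters its box, it marks itself discovered, notifies that player's HUD the first time, and updates the checkpoint through the player state on every entry.
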(event `self.ReceiveBeginPlay`
  (bind _aswbp_tag (cast `/Game/SurvivalGame/GroupSystem/WBP_Tag` (`WidgetComponent.GetWidget` (`self.Widget`)) :!pure true))
  (`KismetArrayLibrary.Array_AddUnique` (`/Game/SurvivalGame/BP_CustomGameState.TravelLocations` (cast `/Game/SurvivalGame/BP_CustomGameState` (`GameplayStatics.GetGameState`) :!pure true)) self)
  (set `/Game/SurvivalGame/GroupSystem/WBP_Tag.TagAttached` self _aswbp_tag)
  (`/Game/SurvivalGame/GroupSystem/WBP_Tag.RefreshTag` _aswbp_tag))

(event `ToggleWidgetVisibility`
  (params (ShouldShowWidget :type Boolean))
  (`SceneComponent.SetHiddenInGame` (`self.Widget`) (not ShouldShowWidget) false)
  (`/Game/SurvivalGame/GroupSystem/WBP_Tag.RefreshTag` (cast `/Game/SurvivalGame/GroupSystem/WBP_Tag` (`WidgetComponent.GetWidget` (`self.Widget`)) :!pure true)))

(event `self.Box.OnComponentBeginOverlap`
  (params (OverlappedComponent :type "PrimitiveComponent Object Reference") (OtherActor :type "Actor Object Reference") (OtherComp :type "PrimitiveComponent Object Reference") (OtherBodyIndex :type Integer) (bFromSweep :type Boolean) (SweepResult :type "HitResult Structure (by ref)"))
  (bind _asbp_third_person_character (cast `/Game/StarterPack/ThirdPerson/Blueprints/BP_ThirdPersonCharacter` OtherActor))
  (if (`Pawn.IsLocallyControlled` _asbp_third_person_character)
    (if (not (`self.IsDiscovered`))
      (set `self.IsDiscovered` true)
      (`/Game/SurvivalGame/WBP_HUD.DiscoverNewLocation` (`/Game/StarterPack/ThirdPerson/Blueprints/BP_ThirdPersonCharacter.HUD_Ref` _asbp_third_person_character) self))
    (`/Game/SurvivalGame/BP_CustomPlayerState.S_UpdateCheckpoint` (cast `/Game/SurvivalGame/BP_CustomPlayerState` (`Pawn.PlayerState` _asbp_third_person_character) :!pure true) self)))

(fn `UserConstructionScript`)