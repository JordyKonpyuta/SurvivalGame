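; BP_ItemObject represents a single inventory item, holding its index, data and rotation state.
; OC_SetItemData stores the index and uses it as the row name to load ItemData from DT_Items.
; Rotate toggles the rotation flag, which makes GetDimensions swap X and Y and GetIcon return the rotated material.
; Getter functions expose the data, index and rotation state.
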(event `OC_SetItemData`
  (params (Index :type Integer))
  (bind _output_get (set `self.Index` Index))
  (bind _returnvalue (`|GetDataTableRow` "/Game/SurvivalGame/InventorySystem/Items/DT_Items.DT_Items" (`KismetStringLibrary.Conv_StringToName` (`KismetStringLibrary.Conv_IntToString` _output_get)))
    (:`then`
      (set `self.ItemData` _returnvalue))))

(fn `GetDimensions`
  (returns (Dimensions :type "IntPoint Structure"))
  (bind ((`Dimensions_2_6AF197CF4574540F6830A08C2E262C3D` _dimensions)) (break `/Game/SurvivalGame/InventorySystem/Items/S_Items` (`self.ItemData`)))
  (if (`self.IsRotated`)
    (return (make `IntPoint` (`.Y` (break `IntPoint` _dimensions)) (break `IntPoint` _dimensions)))
    (else
      (return (`.Dimensions_2_6AF197CF4574540F6830A08C2E262C3D` (break `/Game/SurvivalGame/InventorySystem/Items/S_Items` (`self.ItemData`)))))))

(fn `GetIcon`
  (returns (ReturnValue :type "MaterialInstance Object Reference"))
  (bind ((`Stat1_42_1C91B86D43EAB8001B4000AAD0CFF66B` _stat1) (`Stat2_43_CC56D0FB42AD1FA5A29D78A0263F54F0` _stat2) (`Stat3_44_CA01071D4567F3815CE148A65AA67193` _stat3) (`Material_40_ADE310064552662540E8068F909458A9` _material) (`MaterialRotated_41_0F83DEC14AD51BEE633F3496CBC032DF` _materialrotated)) (break `/Game/SurvivalGame/InventorySystem/Items/S_Items` (`self.ItemData`)))
  (return (select `bool` (`self.IsRotated`) :`false` _material :`true` _materialrotated)))

(fn `GetIndex`
  (returns (Index :type Integer))
  (return (`self.Index`)))

(fn `GetIsRotate`
  (returns (IsRotated :type Boolean))
  (return (`self.IsRotated`)))

(fn `GetItemData`
  (returns (ItemData :type "/Game/SurvivalGame/InventorySystem/Items/S_Items Structure"))
  (return (`self.ItemData`)))

(fn `Rotate`
  (returns (IsRotated :type Boolean))
  (bind _output_get (set `self.IsRotated` (not (`self.IsRotated`))))
  (return _output_get))