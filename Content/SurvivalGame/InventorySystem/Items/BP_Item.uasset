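; BP_Item is a world item pickup that adds itself to a player's inventory on sphere overlap.
; On BeginPlay it builds and initializes a replicated item object from its Index, rebuilding it after a short delay; OnRep_ItemObject applies the mesh from the item data.
; The locally controlled character tries to add the object to its replicated inventory component, then asks its player controller to destroy the actor.
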(event `self.ReceiveTick`
  (params (DeltaSeconds :type "Float (single-precision)")))

(event `self.ReceiveBeginPlay`
  (bind _itemobject (`self.ItemObject`))
  (if (not (`KismetSystemLibrary.IsValid` (`self.ItemObject`)))
    (`self.OC_GetDefaultItemObject`))
  (`self.OC_InitializeObject` _itemobject)
  (`KismetSystemLibrary.Delay` 2.0)
  (`self.OC_GetDefaultItemObject`)
  (`self.OC_InitializeObject` _itemobject))

(event `self.Sphere.OnComponentBeginOverlap`
  (params (OverlappedComponent :type "PrimitiveComponent Object Reference") (OtherActor :type "Actor Object Reference") (OtherComp :type "PrimitiveComponent Object Reference") (OtherBodyIndex :type Integer) (bFromSweep :type Boolean) (SweepResult :type "HitResult Structure (by ref)"))
  (bind _asbp_third_person_character (cast `/Game/StarterPack/ThirdPerson/Blueprints/BP_ThirdPersonCharacter` OtherActor))
  (if (`Pawn.IsLocallyControlled` _asbp_third_person_character)
    (bind _inventorycomponent_replicated (`/Game/StarterPack/ThirdPerson/Blueprints/BP_ThirdPersonCharacter.InventoryComponent_Replicated` _asbp_third_person_character))
    (bind (_added _topleftindex _itemobjecttoadd) (`/Game/SurvivalGame/InventorySystem/BP_InventoryComponent_Replicated.TryAddItem` _inventorycomponent_replicated (`self.ItemObject`)))
    (if _added
      (`/Game/SurvivalGame/InventorySystem/BP_InventoryComponent_Replicated.OC_AddItemAtIndex` _inventorycomponent_replicated _topleftindex _itemobjecttoadd)
      (`/Game/StarterPack/ThirdPerson/Blueprints/BP_ThirdPersonPlayerController.S_RequestDestroyItem` (cast `/Game/StarterPack/ThirdPerson/Blueprints/BP_ThirdPersonPlayerController` (`Pawn.GetController` _asbp_third_person_character) :!pure true) self))))

(event `OC_InitializeObject`
  (params (ItemObject :type "/Game/SurvivalGame/InventorySystem/Items/BP_ItemObject_Replicated Object Reference"))
  (bind _output_get (set `self.ItemObject` ItemObject))
  (`/Game/SurvivalGame/InventorySystem/Items/BP_ItemObject_Replicated.OC_SetItemData` _output_get (`/Game/SurvivalGame/InventorySystem/Items/BP_ItemObject_Replicated.GetIndex` _output_get))
  (set `self.ItemData` (`/Game/SurvivalGame/InventorySystem/Items/BP_ItemObject_Replicated.GetItemData` _output_get)))

(event `OC_GetDefaultItemObject`
  (bind _returnvalue (`|GenericCreateObject` "/Game/SurvivalGame/InventorySystem/Items/BP_ItemObject_Replicated.BP_ItemObject_Replicated_C" (`self.Index`)))
  (set `self.ItemObject` _returnvalue))

(fn `OnRep_ItemObject`
  (`StaticMeshComponent.SetStaticMesh` (`self.StaticMesh`) (`.Mesh_30_335522894BA715DBBB818E8F43EE56D5` (break `/Game/SurvivalGame/InventorySystem/Items/S_Items` (`self.ItemData`)))))

(fn `UserConstructionScript`)