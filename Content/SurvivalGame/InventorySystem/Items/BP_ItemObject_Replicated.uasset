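; Inventory item object that holds one item's index, data table row and rotation state for the survival game's inventory.
; OC_SetItemData stores the index and uses it as the row name to load ItemData from DT_Items.
; Rotate toggles IsRotated, which makes GetDimensions swap X and Y and GetIcon return the rotated material.
; Simple getters expose the data, index and rotation state.
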(event `OC_SetItemData`
  (params (Index :type Integer))
  (bind _output_get (set `self.Index` Index))
  (bind _returnvalue (`|GetDataTableRow` "/Game/SurvivalGame/InventorySystem/Items/DT_Items.DT_Items" (`KismetStringLibrary.Conv_StringToName` (`KismetStringLibrary.Conv_IntToString` _output_get)))
    (:`then`
      (set `self.ItemData` _returnvalue))))

(fn `GetDimensions`
  (returns (Dimensions :type "IntPoint Structure"))
  (bind (_x _y) (break `IntPoint` (`.Dimensions_2_6AF197CF4574540F6830A08C2E262C3D` (break `/Game/SurvivalGame/InventorySystem/Items/S_Items` (`self.ItemData`)))))
  (if (`self.IsRotated`)
    (return (make `IntPoint` _y _x))
    (else
      (return (`.Dimensions_2_6AF197CF4574540F6830A08C2E262C3D` (break `/Game/SurvivalGame/InventorySystem/Items/S_Items` (`self.ItemData`)))))))

(fn `GetIcon`
  (returns (ReturnValue :type "MaterialInstance Object Reference"))
  (bind ((`Material_40_ADE310064552662540E8068F909458A9` _material) (`MaterialRotated_41_0F83DEC14AD51BEE633F3496CBC032DF` _materialrotated)) (break `/Game/SurvivalGame/InventorySystem/Items/S_Items` (`self.ItemData`)))
  (return (select `bool` (`self.IsRotated`) :`false` _material :`true` _materialrotated)))

(fn `GetIndex`
  (returns (Index :type Integer))
  (return (`self.Index`)))

(fn `GetIsRotate`
  (returns (IsRotated :type Boolean))
  (return (`self.IsRotated`)))

(fn `GetItemData`
  (returns (ItemData :type "/Game/SurvivalGame/InventorySystem/Items/S_Items Structure"))
  (return (`self.ItemData`)))

(fn `Rotate`
  (returns (IsRotated :type Boolean))
  (bind _output_get (set `self.IsRotated` (not (`self.IsRotated`))))
  (return _output_get))