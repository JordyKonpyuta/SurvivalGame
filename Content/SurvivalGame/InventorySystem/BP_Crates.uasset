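; BP_Crates is a lootable container actor for the survival inventory system that appears as either a backpack or a crate.
; On BeginPlay it sets mesh, scale and offset from IsBackbag, and only crates get random loot.
; Loot items are replicated objects with random DT_Items indices, capped by the numeric last row name, added where InventoryComponent finds space.
; Sphere overlaps set or clear InteractableCrate on the locally controlled character.
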(event `self.ReceiveBeginPlay`
  (`StaticMeshComponent.SetStaticMesh` (`self.StaticMesh`) (select `bool` (`self.IsBackbag`) :`false` "/Game/Assets/Fab/Crate_-_Low_poly_count__Stylized_Textures/crate_low_poly_count_stylized_textures/StaticMeshes/crate_low_poly_count_stylized_textures.crate_low_poly_count_stylized_textures" :`true` "/Game/Assets/Fab/Stylized_3D_Backpack/back_pack/StaticMeshes/back_pack.back_pack" :!type "StaticMesh Object Reference"))
  (`SceneComponent.SetWorldScale3D` (`self.StaticMesh`) (select `bool` (`self.IsBackbag`) :`false` (1.0 1.0 1.0) :`true` (0.01 0.01 0.01) :!type "Vector Structure"))
  (`SceneComponent.K2_SetRelativeLocation` (`self.StaticMesh`) (select `bool` (`self.IsBackbag`) :`false` (0.0 0.0 50.0) :`true` (0.0 0.0 -10.0) :!type "Vector Structure") false false)
  (if (not (`self.IsBackbag`))
    (`self.OC_SetObjectsInCrate`)))

(event `OC_SetObjectsInCrate`
  (for _ (range (+ (`KismetMathLibrary.RandomIntegerInRange` 0 5) 1))
    (bind _outrownames (`DataTableFunctionLibrary.GetDataTableRowNames` "/Game/SurvivalGame/InventorySystem/Items/DT_Items.DT_Items"))
    (bind _returnvalue (`KismetMathLibrary.RandomIntegerInRange` 0 (`KismetStringLibrary.Conv_StringToInt` (`KismetStringLibrary.Conv_NameToString` (`|GetArrayItem` _outrownames (`KismetArrayLibrary.Array_LastIndex` _outrownames))))))
    (bind _returnvalue_2 (`|GenericCreateObject` "/Game/SurvivalGame/InventorySystem/Items/BP_ItemObject_Replicated.BP_ItemObject_Replicated_C" _returnvalue))
    (`/Game/SurvivalGame/InventorySystem/Items/BP_ItemObject_Replicated.OC_SetItemData` _returnvalue_2 _returnvalue)
    (bind (_added _topleftindex _itemobjecttoadd) (`/Game/SurvivalGame/InventorySystem/BP_InventoryComponent_Replicated.TryAddItem` (`self.InventoryComponent`) _returnvalue_2))
    (if _added
      (`/Game/SurvivalGame/InventorySystem/BP_InventoryComponent_Replicated.S_AddItemAtIndex` (`self.InventoryComponent`) _topleftindex _itemobjecttoadd))))

(event `self.Sphere.OnComponentBeginOverlap`
  (params (OverlappedComponent :type "PrimitiveComponent Object Reference") (OtherActor :type "Actor Object Reference") (OtherComp :type "PrimitiveComponent Object Reference") (OtherBodyIndex :type Integer) (bFromSweep :type Boolean) (SweepResult :type "HitResult Structure (by ref)"))
  (bind _asbp_third_person_character (cast `/Game/StarterPack/ThirdPerson/Blueprints/BP_ThirdPersonCharacter` OtherActor))
  (if (`Pawn.IsLocallyControlled` _asbp_third_person_character)
    (set `/Game/StarterPack/ThirdPerson/Blueprints/BP_ThirdPersonCharacter.InteractableCrate` self _asbp_third_person_character)))

(event `self.Sphere.OnComponentEndOverlap`
  (params (OverlappedComponent :type "PrimitiveComponent Object Reference") (OtherActor :type "Actor Object Reference") (OtherComp :type "PrimitiveComponent Object Reference") (OtherBodyIndex :type Integer))
  (bind _asbp_third_person_character (cast `/Game/StarterPack/ThirdPerson/Blueprints/BP_ThirdPersonCharacter` OtherActor))
  (if (`Pawn.IsLocallyControlled` _asbp_third_person_character)
    (set `/Game/StarterPack/ThirdPerson/Blueprints/BP_ThirdPersonCharacter.InteractableCrate` null _asbp_third_person_character)))

(fn `UserConstructionScript`)