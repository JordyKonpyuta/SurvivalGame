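; Replicated grid inventory component that stores multi-tile items in a flat Columns × Rows array, with each item filling every tile it covers.
; TryAddItem scans for free, in-bounds space, retrying with the item rotated, and returns the index that OC_AddItemAtIndex fills.
; Adds and removals set IsDirty, whose OnRep refreshes the ThirdPersonCharacter's inventory grid widget.
; Other events empty the inventory or consume items to raise Health, Hunger and Thirst.
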(event `self.ReceiveBeginPlay`
  (`KismetArrayLibrary.Array_Resize` (`self.AllItems`) (* (`self.Columns`) (`self.Rows`))))

(event `OC_AddItemAtIndex`
  (params (TopLeftIndex :type Integer) (ItemObject :type "/Game/SurvivalGame/InventorySystem/Items/BP_ItemObject_Replicated Object Reference"))
  (bind _tile (`self.ForEachIndex` TopLeftIndex ItemObject)
    (:`LoopBody`
      (`KismetArrayLibrary.Array_Set` (`self.AllItems`) (`self.TileToIndex` _tile) ItemObject true))
    (:`Completed`
      (set `self.IsDirty` true))))

(event `OC_OnInventoryChange`
  (bind _asbp_third_person_character (cast `/Game/StarterPack/ThirdPerson/Blueprints/BP_ThirdPersonCharacter` (`self.GetOwner`)))
  (`/Game/SurvivalGame/InventorySystem/WBP_InventoryGrid.RefreshInventory` (`/Game/SurvivalGame/InventorySystem/WBP_Inventory.WBP_InventoryGrid` (`/Game/StarterPack/ThirdPerson/Blueprints/BP_ThirdPersonCharacter.InventoryUI` _asbp_third_person_character))))

(event `OC_UseConsumable`
  (params (ItemObject :type "/Game/SurvivalGame/InventorySystem/Items/BP_ItemObject_Replicated Object Reference"))
  (bind ((`Stat1_42_1C91B86D43EAB8001B4000AAD0CFF66B` _stat1) (`Stat2_43_CC56D0FB42AD1FA5A29D78A0263F54F0` _stat2) (`Stat3_44_CA01071D4567F3815CE148A65AA67193` _stat3)) (break `/Game/SurvivalGame/InventorySystem/Items/S_Items` (`/Game/SurvivalGame/InventorySystem/Items/BP_ItemObject_Replicated.GetItemData` ItemObject)))
  (bind _asbp_third_person_character (cast `/Game/StarterPack/ThirdPerson/Blueprints/BP_ThirdPersonCharacter` (`self.GetOwner`) :!pure true))
  (set `/Game/StarterPack/ThirdPerson/Blueprints/BP_ThirdPersonCharacter.Health` (+ (`/Game/StarterPack/ThirdPerson/Blueprints/BP_ThirdPersonCharacter.Health` _asbp_third_person_character) _stat1) _asbp_third_person_character)
  (set `/Game/StarterPack/ThirdPerson/Blueprints/BP_ThirdPersonCharacter.Hunger` (+ (`/Game/StarterPack/ThirdPerson/Blueprints/BP_ThirdPersonCharacter.Hunger` _asbp_third_person_character) _stat2) _asbp_third_person_character)
  (set `/Game/StarterPack/ThirdPerson/Blueprints/BP_ThirdPersonCharacter.Thirst` (+ (`/Game/StarterPack/ThirdPerson/Blueprints/BP_ThirdPersonCharacter.Thirst` _asbp_third_person_character) _stat3) _asbp_third_person_character)
  (`self.RemoveItem` ItemObject))

(event `OC_EmptyInventory`
  (bind _allitems (`self.GetAllItems`))
  (bind _keys (`BlueprintMapLibrary.Map_Keys` _allitems))
  (for _array_element _keys
    (`self.RemoveItem` _array_element)))

(fn `GetAllItems`
  (returns (AllItems :type "Map of /Game/SurvivalGame/InventorySystem/Items/BP_ItemObject_Replicated Object Reference to /Game/SurvivalGame/InventorySystem/S_Tile Structure"))
  (locals (TempAllItems :type "Map of /Game/SurvivalGame/InventorySystem/Items/BP_ItemObject_Replicated Object Reference to /Game/SurvivalGame/InventorySystem/S_Tile Structure") (CurrentItem :type "/Game/SurvivalGame/InventorySystem/Items/BP_ItemObject_Replicated Object Reference"))
  (for (_array_element _array_index) (`self.AllItems`)
    (bind _asbp_item_object_replicated (cast `/Game/SurvivalGame/InventorySystem/Items/BP_ItemObject_Replicated` _array_element))
    (bind _output_get (set `local.CurrentItem` _asbp_item_object_replicated))
    (`/Engine/EditorBlueprintResources/StandardMacros.IsValid` _output_get
      (:`Is Valid`
        (if (not (`BlueprintMapLibrary.Map_Contains` (`local.TempAllItems`) _output_get))
          (`BlueprintMapLibrary.Map_Add` (`local.TempAllItems`) (`local.CurrentItem`) (`self.IndexToTile` _array_index))))))
  (return (`local.TempAllItems`)))

(fn `GetItemAtIndex`
  (params (Index :type Integer))
  (returns (Valid :type Boolean) (ItemObject :type "/Game/SurvivalGame/InventorySystem/Items/BP_ItemObject_Replicated Object Reference"))
  (if (`KismetArrayLibrary.Array_IsValidIndex` (`self.AllItems`) Index)
    (return true (cast `/Game/SurvivalGame/InventorySystem/Items/BP_ItemObject_Replicated` (`|GetArrayItem` (`self.AllItems`) (`local.Index`)) :!pure true))
    (else
      (return false null))))

(fn `IndexToTile`
  (params (Index :type Integer))
  (returns (Tile :type "/Game/SurvivalGame/InventorySystem/S_Tile Structure"))
  (return (make `/Game/SurvivalGame/InventorySystem/S_Tile` (mod Index (`self.Columns`)) (/ Index (`self.Columns`)))))

(fn `IsRoomAvailable`
  (params (ItemObject :type "/Game/SurvivalGame/InventorySystem/Items/BP_ItemObject_Replicated Object Reference") (TopLeftIndex :type Integer))
  (returns (Result :type Boolean))
  (`|ExecutionSequence`
    (:`then_0`
      (bind _tile (`self.ForEachIndex` (`local.TopLeftIndex`) (`local.ItemObject`))
        (:`LoopBody`
          (`self.IsTileValid` _tile
            (:`true`
              (bind (_valid _itemobject) (`self.GetItemAtIndex` (`self.TileToIndex` _tile)))
              (if _valid
                (if (`KismetSystemLibrary.IsValid` _itemobject)
                  (`KismetSystemLibrary.PrintString` "Room not available")
                  (return false))
                (else
                  (`KismetSystemLibrary.PrintString` "Invalid Index")
                  (return false))))
            (:`false`
              (`KismetSystemLibrary.PrintString` "No Tile Valid")
              (return false))))))
    (:`then_1`
      (return true))))

(fn `OnRep_IsDirty`
  (if (`self.IsDirty`)
    (set `self.IsDirty` false)
    (`self.OC_OnInventoryChange`)))

(fn `RemoveItem`
  (params (ItemObject :type "/Game/SurvivalGame/InventorySystem/Items/BP_ItemObject_Replicated Object Reference"))
  (`/Engine/EditorBlueprintResources/StandardMacros.IsValid` ItemObject
    (:`Is Valid`
      (for (_array_element _array_index) (`self.AllItems`)
        (if (== _array_element (`local.ItemObject`))
          (`KismetArrayLibrary.Array_Set` (`self.AllItems`) _array_index null true)
          (set `self.IsDirty` true))))))

(fn `TileToIndex`
  (params (Tile :type "/Game/SurvivalGame/InventorySystem/S_Tile Structure"))
  (returns (Index :type Integer))
  (bind (_x _y) (break `/Game/SurvivalGame/InventorySystem/S_Tile` Tile))
  (return (+ _x (* _y (`self.Columns`)))))

(fn `TryAddItem`
  (params (ItemObject :type "/Game/SurvivalGame/InventorySystem/Items/BP_ItemObject_Replicated Object Reference"))
  (returns (Added :type Boolean) (TopLeftIndex :type Integer) (ItemObjectToAdd :type "/Game/SurvivalGame/InventorySystem/Items/BP_ItemObject_Replicated Object Reference"))
  (`/Engine/EditorBlueprintResources/StandardMacros.IsValid` ItemObject
    (:`Is Valid`
      (for (_ _array_index) (`self.AllItems`) :!label _label
        (bind _result (`self.IsRoomAvailable` (`local.ItemObject`) _array_index))
        (if _result
          (return true _array_index (`local.ItemObject`))))
      (`|ExecutionSequence`
        (:`then_0`
          (`/Engine/EditorBlueprintResources/StandardMacros.DoOnce` false
            (:`Completed`
              (`/Game/SurvivalGame/InventorySystem/Items/BP_ItemObject_Replicated.Rotate` (`local.ItemObject`))
              (goto _label))))
        (:`then_1`
          (`/Game/SurvivalGame/InventorySystem/Items/BP_ItemObject_Replicated.Rotate` (`local.ItemObject`))
          (`KismetSystemLibrary.PrintString` "Nope")
          (return false 0 null))))
    (:`Is Not Valid`
      (`KismetSystemLibrary.PrintString` "No Object"))))