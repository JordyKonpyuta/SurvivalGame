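; Equipment component that tracks items in a fixed number of slots and the Attack, AttackSpeed and Defense stats they grant.
; S_ add and remove events set or clear a slot, then adjust stats by Weapon or Armor type; removing Armor adds to Defense instead of subtracting.
; RepNotify functions on each stat push truncated values to the equipment grid text in the owning BP_ThirdPersonCharacter's inventory UI.
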(event `self.ReceiveBeginPlay`
  (`KismetArrayLibrary.Array_Resize` (`self.Equipments`) (`self.EquipmentSlots`)))

(event `S_RemoveEquipmentAtIndex`
  (params (Index :type Integer) (ItemObject :type "/Game/SurvivalGame/InventorySystem/Items/BP_ItemObject_Replicated Object Reference"))
  (bind ((`ItemType_21_2C4A3BEE44C498B36B34D1A5E4124EB7` _itemtype) (`Stat1_42_1C91B86D43EAB8001B4000AAD0CFF66B` _stat1) (`Stat2_43_CC56D0FB42AD1FA5A29D78A0263F54F0` _stat2) (`Stat3_44_CA01071D4567F3815CE148A65AA67193` _stat3)) (break `/Game/SurvivalGame/InventorySystem/Items/S_Items` (`/Game/SurvivalGame/InventorySystem/Items/BP_ItemObject_Replicated.GetItemData` ItemObject)))
  (`|ExecutionSequence`
    (:`then_0`
      (`KismetArrayLibrary.Array_Set` (`self.Equipments`) Index null true))
    (:`then_1`
      (switch `/Game/SurvivalGame/InventorySystem/Items/E_ItemType` _itemtype
        (:`NewEnumerator0`
          (set `self.Attack` (- (`self.Attack`) _stat1))
          (set `self.AttackSpeed` (- (`self.AttackSpeed`) _stat2)))
        (:`NewEnumerator1`
          (set `self.Defense` (+ (`self.Defense`) _stat3)))))))

(event `S_AddEquipmentAtIndex`
  (params (Index :type Integer) (ItemObject :type "/Game/SurvivalGame/InventorySystem/Items/BP_ItemObject_Replicated Object Reference"))
  (bind ((`ItemType_21_2C4A3BEE44C498B36B34D1A5E4124EB7` _itemtype) (`Stat1_42_1C91B86D43EAB8001B4000AAD0CFF66B` _stat1) (`Stat2_43_CC56D0FB42AD1FA5A29D78A0263F54F0` _stat2) (`Stat3_44_CA01071D4567F3815CE148A65AA67193` _stat3)) (break `/Game/SurvivalGame/InventorySystem/Items/S_Items` (`/Game/SurvivalGame/InventorySystem/Items/BP_ItemObject_Replicated.GetItemData` ItemObject)))
  (`|ExecutionSequence`
    (:`then_0`
      (`KismetArrayLibrary.Array_Set` (`self.Equipments`) Index ItemObject true))
    (:`then_1`
      (switch `/Game/SurvivalGame/InventorySystem/Items/E_ItemType` _itemtype
        (:`NewEnumerator0`
          (set `self.Attack` (+ (`self.Attack`) _stat1))
          (set `self.AttackSpeed` (+ (`self.AttackSpeed`) _stat2)))
        (:`NewEnumerator1`
          (set `self.Defense` (+ (`self.Defense`) _stat3)))))))

(fn `OnRep_Attack`
  (bind _asbp_third_person_character (cast `/Game/StarterPack/ThirdPerson/Blueprints/BP_ThirdPersonCharacter` (`self.GetOwner`)))
  (`TextBlock.SetText` (`/Game/SurvivalGame/EquipmentSystem/WBP_EquipmentGrid.Text_Attack` (`/Game/SurvivalGame/InventorySystem/WBP_Inventory.WBP_EquipmentGrid` (`/Game/StarterPack/ThirdPerson/Blueprints/BP_ThirdPersonCharacter.InventoryUI` _asbp_third_person_character))) (`KismetTextLibrary.Conv_IntToText` (`KismetMathLibrary.FTrunc` (`self.Attack`)))))

(fn `OnRep_AttackSpeed`
  (bind _asbp_third_person_character (cast `/Game/StarterPack/ThirdPerson/Blueprints/BP_ThirdPersonCharacter` (`self.GetOwner`)))
  (`TextBlock.SetText` (`/Game/SurvivalGame/EquipmentSystem/WBP_EquipmentGrid.Text_AttackSpeed` (`/Game/SurvivalGame/InventorySystem/WBP_Inventory.WBP_EquipmentGrid` (`/Game/StarterPack/ThirdPerson/Blueprints/BP_ThirdPersonCharacter.InventoryUI` _asbp_third_person_character))) (`KismetTextLibrary.Conv_IntToText` (`KismetMathLibrary.FTrunc` (`self.AttackSpeed`)))))

(fn `OnRep_Defense`
  (bind _asbp_third_person_character (cast `/Game/StarterPack/ThirdPerson/Blueprints/BP_ThirdPersonCharacter` (`self.GetOwner`)))
  (`TextBlock.SetText` (`/Game/SurvivalGame/EquipmentSystem/WBP_EquipmentGrid.Text_Defense` (`/Game/SurvivalGame/InventorySystem/WBP_Inventory.WBP_EquipmentGrid` (`/Game/StarterPack/ThirdPerson/Blueprints/BP_ThirdPersonCharacter.InventoryUI` _asbp_third_person_character))) (`KismetTextLibrary.Conv_IntToText` (`KismetMathLibrary.FTrunc` (`self.Defense`)))))