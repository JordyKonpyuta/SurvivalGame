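; Camera actor for the character customisation screen that frames the body area matching the selected clothing category.
; On BeginPlay it becomes the view target, registers as the player character's preview, opens the customisation widget and switches to UI-only input with the cursor shown.
; CameraMovement stores the category and starts a looping timer that interpolates the camera toward that category's arrow component, clearing itself once the transforms nearly match.
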(event `self.ReceiveBeginPlay`
  (bind _returnvalue (`GameplayStatics.GetPlayerController` 0))
  (bind _asbp_third_person_character (cast `/Game/StarterPack/ThirdPerson/Blueprints/BP_ThirdPersonCharacter` (`GameplayStatics.GetPlayerCharacter` 0) :!pure true))
  (`PlayerController.SetViewTargetWithBlend` (`GameplayStatics.GetPlayerController` 0) self 0.0 "VTBlend_Linear" 0.0 false)
  (bind _output_get (set `/Game/StarterPack/ThirdPerson/Blueprints/BP_ThirdPersonCharacter.PlayerPreview` self _asbp_third_person_character))
  (bind _returnvalue_2 (`|CreateWidget` "/Game/SurvivalGame/MainMenu/CharacterCustomisation/WBP_CharacterCustomisation.WBP_CharacterCustomisation_C" null _output_get _asbp_third_person_character))
  (`UserWidget.AddToViewport` _returnvalue_2 0)
  (`WidgetBlueprintLibrary.SetInputMode_UIOnlyEx` _returnvalue _returnvalue_2 "DoNotLock" true)
  (set `PlayerController.bShowMouseCursor` true _returnvalue))

(event `MoveCamera`
  (bind _returnvalue (`SceneComponent.GetRelativeTransform` (`self.Camera`)))
  (bind _returnvalue_2 (`SceneComponent.GetRelativeTransform` (select `/Game/SurvivalGame/MainMenu/CharacterCustomisation/E_ClothPieces` (`self.Cloth Category`) :`NewEnumerator3` (`self.Arrow_Hair`) :`NewEnumerator4` (`self.Arrow_Start`) :`NewEnumerator2` (`self.Arrow_Dress`) :`NewEnumerator0` (`self.Arrow_Top`) :`NewEnumerator1` (`self.Arrow_Bottom`) :`NewEnumerator5` (`self.Arrow_Shoes`) :`NewEnumerator6` (`self.Arrow_Accessory`) :`NewEnumerator7` (`self.Arrow_Ears`) :`NewEnumerator8` (`self.Arrow_Tail`) :`NewEnumerator9` (`self.Arrow_Eyes`) :!type "SceneComponent Object Reference")))
  (`SceneComponent.K2_SetRelativeTransform` (`self.Camera`) (`KismetMathLibrary.TInterpTo` _returnvalue _returnvalue_2 (`GameplayStatics.GetWorldDeltaSeconds`) 2.0) false false)
  (if (`KismetMathLibrary.NearlyEqual_TransformTransform` _returnvalue _returnvalue_2)
    (`KismetSystemLibrary.K2_ClearAndInvalidateTimerHandle` (`self.CameraMovementTimerHandle`))))

(event `CameraMovement`
  (params (ClothCategory :type "/Game/SurvivalGame/MainMenu/CharacterCustomisation/E_ClothPieces Enum" :default "NewEnumerator3"))
  (set `self.Cloth Category` ClothCategory)
  (bind _returnvalue (`KismetSystemLibrary.K2_SetTimerDelegate` (`|CreateDelegate` :!event `MoveCamera`) 0.01 true))
  (set `self.CameraMovementTimerHandle` _returnvalue))

(fn `UserConstructionScript`)