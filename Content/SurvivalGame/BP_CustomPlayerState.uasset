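; Custom player state for the survival game that stores the player's last visited checkpoint and group members, and controls player tag visibility.
; BeginPlay sets the first travel location as the checkpoint and adds the player to its own group.
; Prefixed server and owning-client events relay group requests and edit membership, firing OnGroupChanged.
; When tags are enabled, they show for self and group members only.
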(event `self.ReceiveBeginPlay`
  (`self.S_UpdateCheckpoint` (`|GetArrayItem` (`self.TravelLocations`)))
  (`KismetArrayLibrary.Array_AddUnique` (`self.PlayersInGroup`) self))

(event `S_UpdateCheckpoint`
  (params (LastVisitedLocation :type "/Game/SurvivalGame/GroupSystem/BP_Tag Object Reference"))
  (set `self.LastVisitedLocation` LastVisitedLocation))

(event `S_RequestGroup`
  (params (Target :type "/Game/SurvivalGame/BP_CustomPlayerState Object Reference") (PlayerToAdd :type "/Game/SurvivalGame/BP_CustomPlayerState Object Reference"))
  (`self.OC_AddPlayerToGroup` Target PlayerToAdd))

(event `OC_AddPlayerToGroup`
  (params (PlayerToAdd :type "/Game/SurvivalGame/BP_CustomPlayerState Object Reference"))
  (`KismetArrayLibrary.Array_AddUnique` (`self.PlayersInGroup`) PlayerToAdd)
  (`KismetArrayLibrary.Array_AddUnique` (`self.PlayersInGroup`) self)
  (`self.OnGroupChanged`))

(event `OC_RemovePlayerFromGroup`
  (params (PlayerToRemove :type "/Game/SurvivalGame/BP_CustomPlayerState Object Reference"))
  (`KismetArrayLibrary.Array_RemoveItem` (`self.PlayersInGroup`) PlayerToRemove)
  (`self.OnGroupChanged`))

(event `OC_ToggleTagsVisibility`
  (params (PlayerState :type "/Game/SurvivalGame/BP_CustomPlayerState Object Reference") (ShouldShowWidget :type Boolean) (IsSelf :type Boolean))
  (`SceneComponent.SetHiddenInGame` (`/Game/SurvivalGame/BP_CustomPlayerState.PlayerTag` PlayerState) (select `bool` IsSelf :`false` (select `bool` ShouldShowWidget :`false` true :`true` (not (`KismetArrayLibrary.Array_Contains` (`self.PlayersInGroup`) PlayerState))) :`true` (not ShouldShowWidget)) false))

(fn `UserConstructionScript`)