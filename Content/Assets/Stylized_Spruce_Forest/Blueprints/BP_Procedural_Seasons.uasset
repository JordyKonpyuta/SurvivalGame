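; BP_Procedural_Seasons cycles the Stylized Spruce Forest through autumn and winter on an endless, Delay-timed loop started at BeginPlay.
; The loop toggles target values, and Tick calls SeasonUpdate to step the matching MPC_Global scalar parameters toward them by a fixed, frame-rate-dependent amount.
; Niagara logic for rain, falling leaves and snow is present but unconnected, so it never runs.
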(event `self.ReceiveBeginPlay`
  ;[1 1 1] Procedural Seasons
  ;;[1 1 1] Use Delay nodes to control the transition time between seasons
  (`KismetSystemLibrary.Delay` 1.0 :!label _label)
  (set `self.Autumn` 1.0)
  (`KismetSystemLibrary.Delay` 10.0)
  (set `self.Autumn` 0.0)
  (set `self.Winter` 1.0)
  (`KismetSystemLibrary.Delay` 5.0)
  (set `self.Winter` 0.0)
  (goto _label))

(event `self.ReceiveTick`
  (params (DeltaSeconds :type "Float (single-precision)"))
  ;[1 1 1] Procedural Seasons
  ;;[1 1 1] Transition Speed Between Seasons
  (`self.Season_Update` "Autumn" (`self.Autumn`)
    (:`OutputPin`
      (`self.Season_Update` "Winter" (`self.Winter`)))))

(fn `UserConstructionScript`)